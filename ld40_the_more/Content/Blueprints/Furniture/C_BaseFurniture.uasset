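; Base furniture actor that can be captured, released, or broken, with breaking adding chaos to the game.
; Break adds its ChaosValue to CE_GameMode_BP and destroys the actor, doing nothing if the game mode cast fails.
; Captured and Released switch between captured and regular colors through ChangeColor, which creates a dynamic material instance on the static mesh and sets its Color parameter.
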(event EventBeginPlay)

(event Collision|EventActorBeginOverlap
  (params (OtherActor :type Actor%20Object%20Reference)))

(event EventTick
  (params (DeltaSeconds :type Float%20%28single-precision%29)))

(fn ConstructionScript)

(fn Break
  (bind _asce_game_mode_bp (Utilities|Casting|CastToCE_GameMode_BP (Game|GetGameMode)))
  (Default|AddChaos _asce_game_mode_bp (Variables|Default|GetChaosValue))
  (Actor|DestroyActor))

(fn Captured
  (CallFunction|ChangeColor (Variables|Default|GetCapturedColor)))

(fn ChangeColor
  (params (Color :type Color%20Structure))
  (bind _staticmesh (Variables|Default|GetStaticMesh))
  (bind _returnvalue (Rendering|Material|CreateDynamicMaterialInstance _staticmesh 0 (Rendering|Material|GetMaterial _staticmesh 0) :!class /Script/Engine.PrimitiveComponent))
  (Rendering|Material|SetVectorParameterValue _returnvalue "Color" (Math|Conversions|ToLinearColor(Color) Color) :!class /Script/Engine.MaterialInstanceDynamic)
  (Rendering|Material|SetMaterial (Variables|Default|GetStaticMesh) 0 _returnvalue))

(fn Released
  (CallFunction|ChangeColor (Variables|Default|GetRegularColor)))