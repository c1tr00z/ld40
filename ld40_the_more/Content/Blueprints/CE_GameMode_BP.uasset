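; Game mode that tracks a chaos level and puts the play HUD widget on screen at BeginPlay.
; AddChaos raises the level only while it is below the maximum, so a single addition can overshoot the cap.
; A looping timer started at BeginPlay calls DecreaseChaos by name to drain the level gradually while it is above zero, with no Tick logic.
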(event EventBeginPlay
  (bind _returnvalue (UserInterface|CreateWidget "/Game/UI/PlayWidget.PlayWidget_C"))
  (UserInterface|Viewport|AddtoViewport _returnvalue 0)
  (Utilities|Time|SetTimerbyFunctionName self "DecreaseChaos" 0.2 true))

(event EventTick
  (params (DeltaSeconds :type Float%20%28single-precision%29)))

(fn ConstructionScript)

(fn AddChaos
  (params (ChaosValue :type Integer))
  (if (> (Math|Conversions|ToFloat(Integer) (Variables|Default|GetMaxChaosLevel)) (Variables|Default|GetChaosLevel))
    (Variables|Default|SetChaosLevel (+ (Math|Conversions|ToFloat(Integer) ChaosValue) (Variables|Default|GetChaosLevel)))))

(fn DecreaseChaos
  (if (< 0.0 (Variables|Default|GetChaosLevel))
    (Variables|Default|SetChaosLevel (- (Variables|Default|GetChaosLevel) 0.1))))