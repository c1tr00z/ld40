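; Music actor that plays a track whose volume follows the game's chaos level.
; Starts its AudioCurveSource component on BeginPlay and restarts it from the beginning on Tick whenever it stops, keeping the music looping.
; Each Tick also reads the chaos percent from CE_GameMode_BP and applies it directly as the volume multiplier.
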(event EventBeginPlay
  (Audio|Components|Audio|Play (Variables|Default|GetAudioCurveSource) 0.0))

(event Collision|EventActorBeginOverlap
  (params (OtherActor :type Actor%20Object%20Reference)))

(event EventTick
  (params (DeltaSeconds :type Float%20%28single-precision%29))
  (bind _audiocurvesource (Variables|Default|GetAudioCurveSource))
  (if (not (Audio|Components|Audio|IsPlaying _audiocurvesource))
    (Audio|Components|Audio|Play _audiocurvesource 0.0))
  (bind _asce_game_mode_bp (Utilities|Casting|CastToCE_GameMode_BP (Game|GetGameMode)))
  (bind _percent (Default|GetChaosPercent _asce_game_mode_bp))
  (Audio|Components|Audio|SetVolumeMultiplier (Variables|Default|GetAudioCurveSource) _percent :!class /Script/Engine.AudioComponent))

(fn ConstructionScript)