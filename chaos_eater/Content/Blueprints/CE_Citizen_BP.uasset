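; Citizen NPC that detects the player and, while the player stays in its box trigger, damages them and lowers chaos every second.
; A one-second timer scales its detection sphere and cylinder with the game mode's chaos percent, and sphere overlaps set SeePlayer.
; It takes target points from its Spawner at start and when hitting another citizen.
; Each damage tick plays a one-shot animation, then restores the animation Blueprint.
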(event OnComponentBeginOverlap(Sphere)
  (params (OverlappedComponent :type Primitive%20Component%20Object%20Reference) (OtherActor :type Actor%20Object%20Reference) (OtherComp :type Primitive%20Component%20Object%20Reference) (OtherBodyIndex :type Integer) (bFromSweep :type Boolean) (SweepResult :type Hit%20Result%20Structure%20%28by%20ref%29))
  (Utilities|Casting|CastToCE_PlayerCharacter_BP OtherActor)
  (Variables|Default|SetSeePlayer true))

(event OnComponentEndOverlap(Sphere)
  (params (OverlappedComponent :type Primitive%20Component%20Object%20Reference) (OtherActor :type Actor%20Object%20Reference) (OtherComp :type Primitive%20Component%20Object%20Reference) (OtherBodyIndex :type Integer))
  (Utilities|Casting|CastToCE_PlayerCharacter_BP OtherActor)
  (Variables|Default|SetSeePlayer false))

(event OnComponentEndOverlap(Box)
  (params (OverlappedComponent :type Primitive%20Component%20Object%20Reference) (OtherActor :type Actor%20Object%20Reference) (OtherComp :type Primitive%20Component%20Object%20Reference) (OtherBodyIndex :type Integer))
  (Utilities|Casting|CastToCE_PlayerCharacter_BP OtherActor)
  (Utilities|Time|ClearTimerbyFunctionName self "Damage"))

(event OnComponentHit(CapsuleComponent)
  (params (HitComponent :type Primitive%20Component%20Object%20Reference) (OtherActor :type Actor%20Object%20Reference) (OtherComp :type Primitive%20Component%20Object%20Reference) (NormalImpulse :type Vector :default "0, 0, 0") (Hit :type Hit%20Result%20Structure%20%28by%20ref%29))
  (Utilities|Casting|CastToCE_Citizen_BP OtherActor)
  (CallFunction|UpdatePoint false))

(event OnComponentBeginOverlap(Box)
  (params (OverlappedComponent :type Primitive%20Component%20Object%20Reference) (OtherActor :type Actor%20Object%20Reference) (OtherComp :type Primitive%20Component%20Object%20Reference) (OtherBodyIndex :type Integer) (bFromSweep :type Boolean) (SweepResult :type Hit%20Result%20Structure%20%28by%20ref%29))
  (Utilities|Casting|CastToCE_PlayerCharacter_BP OtherActor)
  (Utilities|Time|SetTimerbyFunctionName self "Damage" 1.0 true))

(event Custom|E_DamageAnimation
  (bind _mesh (Variables|Character|GetMesh))
  (Components|Animation|PlayAnimation _mesh 0 false)
  (Utilities|FlowControl|Delay 1.0)
  (Components|Animation|SetAnimationMode _mesh "AnimationBlueprint"))

(event EventBeginPlay
  (|CallParentFunction)
  (bind _newparam (CallFunction|GetCEGameMode))
  (Utilities|FlowControl|Delay 0.0)
  (Rendering|Material|SetMaterial (Variables|Character|GetMesh) 0 (Variables|/Game/Blueprints/CE_GameMode_BP.CE_GameMode_BP_C|GetMaterial _newparam))
  (Utilities|Time|SetTimerbyFunctionName self "UpdateRadius" 1.0 true)
  (CallFunction|UpdatePoint true))

(event Collision|EventActorBeginOverlap
  (params (OtherActor :type Actor%20Object%20Reference))
  (|CallParentFunction OtherActor) ; This node is disabled and will not be called.\nDrag off pins to build functionality.
)

(event EventTick
  (params (DeltaSeconds :type Float%20%28single-precision%29))
  (|CallParentFunction DeltaSeconds))

(fn ConstructionScript
  (|CallParentFunction))

(fn UpdateRadius
  (bind _newparam (CallFunction|GetCEGameMode))
  (bind _percent (Default|GetChaosPercent _newparam))
  (Components|Sphere|SetSphereRadius (Variables|Default|GetSphere) (* 32.0 _percent 5e+01) true)
  (Transformation|SetWorldScale3D (Variables|Default|GetCylinder) (Math|Vector|MakeVector (* _percent 32.0) (* _percent 32.0) 0.1)))

(fn UpdatePoint
  (params (Furniture :type Boolean))
  (bind _point (Default|GetPoint (Variables|Default|GetSpawner)))
  (Variables|Default|SetTargetPoint (Math|Vector|MakeVector (.X (Math|Vector|BreakVector _point)) (.Y (Math|Vector|BreakVector _point)) (.z (Transformation|GetWorldLocation (Variables|Default|GetCapsuleComponent))))))

(fn Damage
  (bind _newparam (CallFunction|GetCEGameMode))
  (CallFunction|EDamageAnimation)
  (Default|LowerChaos _newparam 1.0)
  (bind _asce_player_character_bp (Utilities|Casting|CastToCE_PlayerCharacter_BP (Game|GetPlayerCharacter 0)))
  (Default|EDamage _asce_player_character_bp))