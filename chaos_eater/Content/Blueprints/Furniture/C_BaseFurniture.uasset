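; Base furniture actor that registers with the game mode and can be captured, released or broken to add chaos.
; On BeginPlay it creates a dynamic material for its destructible mesh, whose color parameter shows captured or regular state until broken.
; Break adds its chaos value, shatters the mesh along a given direction with a sound, disables box collision, then unregisters and destroys the actor after a short delay.
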(event Custom|E_WaitAndDestroy
  (bind _asce_game_mode_bp (Utilities|Casting|CastToCE_GameMode_BP (Game|GetGameMode)))
  (Default|RemoveFurniture _asce_game_mode_bp self)
  (Utilities|FlowControl|Delay 2.0)
  (Actor|DestroyActor))

(event EventBeginPlay
  (CallFunction|SetupMaterial)
  (CallFunction|ChangeColor (Variables|Default|GetRegularColor))
  (bind _asce_game_mode_bp (Utilities|Casting|CastToCE_GameMode_BP (Game|GetGameMode)))
  (Default|AddFurniture _asce_game_mode_bp self))

(event Collision|EventActorBeginOverlap
  (params (OtherActor :type Actor%20Object%20Reference)))

(event EventTick
  (params (DeltaSeconds :type Float%20%28single-precision%29)))

(fn ConstructionScript)

(fn Break
  (params (From :type Vector))
  (bind _destructible (Variables|Default|GetDestructible))
  (bind _returnvalue (Transformation|GetWorldLocation _destructible))
  (bind _asce_game_mode_bp (Utilities|Casting|CastToCE_GameMode_BP (Game|GetGameMode)))
  (Default|AddChaos _asce_game_mode_bp (Variables|Default|GetChaosValue))
  (Class|DestructibleComponent|ApplyDamage (Variables|Default|GetDestructible) 1e+01 _returnvalue From 1e+04)
  (Audio|PlaySoundatLocation "/Game/Import/Sounds/387434__blosche__hard-hit.387434__blosche__hard-hit" _returnvalue)
  (Collision|SetCollisionEnabled (Variables|Default|GetBox) "NoCollision")
  (CallFunction|EWaitandDestroy)
  (Variables|Default|SetBroken true))

(fn Captured
  (CallFunction|ChangeColor (Variables|Default|GetCapturedColor)))

(fn ChangeColor
  (params (Color :type Color%20Structure))
  (if (and (Utilities|IsValid (Variables|Default|GetMeterial)) (not (Variables|Default|GetBroken)))
    (Rendering|Material|SetVectorParameterValue (Variables|Default|GetMeterial) "Color" (Math|Conversions|ToLinearColor(Color) Color) :!class /Script/Engine.MaterialInstanceDynamic)))

(fn Released
  (CallFunction|ChangeColor (Variables|Default|GetRegularColor)))

(fn SetupMaterial
  (bind _returnvalue (Rendering|Material|CreateDynamicMaterialInstance "/Game/Materials/Furniture.Furniture" :!class /Script/Engine.KismetMaterialLibrary))
  (Rendering|Material|SetMaterial (Variables|Default|GetDestructible) 0 _returnvalue)
  (Variables|Default|SetMeterial _returnvalue))