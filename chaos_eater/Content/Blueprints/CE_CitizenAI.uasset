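; AI controller for CE_Citizen_BP pawns that switches a citizen between chasing the player and moving between target points.
; A looping timer, used instead of Tick, re-issues AIMoveTo from the citizen's CanControl and SeePlayer state.
; It follows the player when seen, otherwise heads to TargetPoint and calls UpdatePoint on arrival.
; When the citizen cannot be controlled, its move destination becomes its own capsule location.
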(event Custom|E_TrackPlayer
  (bind _returnvalue (Pawn|GetControlledPawn))
  (bind _asce_citizen_bp (Utilities|Casting|CastToCE_Citizen_BP _returnvalue))
  (bind _iscancontrol (Default|CanControl _asce_citizen_bp))
  (if _iscancontrol
    (if (Variables|/Game/Blueprints/CE_Citizen_BP.CE_Citizen_BP_C|GetSeePlayer _asce_citizen_bp)
      (AI|AIMoveTo _returnvalue "0, 0, 0" (Game|GetPlayerCharacter 0) 1e+01 false)
      (else
        (AI|AIMoveTo 0 (Variables|/Game/Blueprints/CE_Citizen_BP.CE_Citizen_BP_C|GetTargetPoint _asce_citizen_bp) 0 1e+01 false
          (:OnSuccess
            (Default|UpdatePoint _asce_citizen_bp true)))))
    (else
      (AI|AIMoveTo 0 (Transformation|GetWorldLocation (Variables|/Script/Engine.Character|GetCapsuleComponent _asce_citizen_bp)) 0 5.0 false))))

(event EventBeginPlay
  (Utilities|Time|SetTimerbyFunctionName 0 "E_TrackPlayer" 0.1 true))

(event EventTick
  (params (DeltaSeconds :type Float%20%28single-precision%29)))

(fn ConstructionScript)