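; Citizen spawner actor that populates the area inside its box component with AI-controlled CE_Citizen_BP pawns, up to a maximum count.
; On BeginPlay it registers itself with CE_GameMode_BP through InitSpawner.
; CheckAndSpawn calls SpawnCitizen while the count is below MaxCitizens, adding one citizen per call at a random point in the box.
; Each spawned citizen receives a reference back to its spawner and increments the count.
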(event EventBeginPlay
  (bind _asce_game_mode_bp (Utilities|Casting|CastToCE_GameMode_BP (Game|GetGameMode)))
  (Default|InitSpawner _asce_game_mode_bp self))

(event Collision|EventActorBeginOverlap
  (params (OtherActor :type Actor%20Object%20Reference)))

(event EventTick
  (params (DeltaSeconds :type Float%20%28single-precision%29)))

(fn ConstructionScript)

(fn GetPoint
  (return (Math|Random|RandomPointinBoundingBox (Transformation|GetWorldLocation (Variables|Default|GetDefaultSceneRoot)) (Components|Box|GetScaledBoxExtent (Variables|Default|GetBox)))))

(fn SpawnCitizen
  (bind _point (CallFunction|GetPoint))
  (bind _returnvalue (AI|SpawnAIFromClass "/Game/Blueprints/CE_Citizen_BP.CE_Citizen_BP_C" 0 _point "0, 0, 0" false))
  (bind _asce_citizen_bp (Utilities|Casting|CastToCE_Citizen_BP _returnvalue))
  (Variables|/Game/Blueprints/CE_Citizen_BP.CE_Citizen_BP_C|SetSpawner _asce_citizen_bp self)
  (bind _result (Math|Integer|IncrementInt (Variables|Default|GetCitizens))
    (:%20%20
      (Variables|Default|SetCitizens _result))))

(fn CheckandSpawn
  (if (> (Variables|Default|GetMaxCitizens) (Variables|Default|GetCitizens))
    (CallFunction|SpawnCitizen)))