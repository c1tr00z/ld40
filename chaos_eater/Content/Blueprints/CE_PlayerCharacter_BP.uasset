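; Player character for a furniture-smashing game, with movement, orbit camera and hit feedback.
; Move input turns the controller toward the stick direction offset by spring arm rotation and moves along its forward; look input rotates the pitch-limited arm.
; Box overlaps mark furniture; pressing Crush captures it, releasing plays an animation and breaks it along the character's forward vector.
; Damage plays a hurt sound and briefly widens camera FOV.
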(event OnComponentBeginOverlap(Box)
  (params (OverlappedComponent :type Primitive%20Component%20Object%20Reference) (OtherActor :type Actor%20Object%20Reference) (OtherComp :type Primitive%20Component%20Object%20Reference) (OtherBodyIndex :type Integer) (bFromSweep :type Boolean) (SweepResult :type Hit%20Result%20Structure%20%28by%20ref%29))
  (bind _asc_base_furniture (Utilities|Casting|CastToC_BaseFurniture OtherActor))
  (Default|Captured _asc_base_furniture)
  (Variables|Default|SetSelectedFurniture _asc_base_furniture))

(event OnComponentEndOverlap(Box)
  (params (OverlappedComponent :type Primitive%20Component%20Object%20Reference) (OtherActor :type Actor%20Object%20Reference) (OtherComp :type Primitive%20Component%20Object%20Reference) (OtherBodyIndex :type Integer))
  (bind _asc_base_furniture (Utilities|Casting|CastToC_BaseFurniture OtherActor))
  (Default|Released _asc_base_furniture)
  (Variables|Default|SetSelectedFurniture 0))

(event Custom|E_RotateTo
  (params (TargetRotator :type Rotator))
  ;[1 1 1] Rotation Event
  (Pawn|SetControlRotation (Pawn|GetController) (Math|Interpolation|RInterpTo (Pawn|GetControlRotation :!class /Script/Engine.Pawn) TargetRotator 0.5 0.3)))

(event Custom|E_Damage
  (bind _camera (Variables|Default|GetCamera))
  (Audio|PlaySoundatLocation "/Game/Import/Sounds/44429__thecheeseman__hurt2.44429__thecheeseman__hurt2" (Transformation|GetWorldLocation (Variables|Default|GetCapsuleComponent)))
  (Camera|SetFieldOfView _camera 95.0)
  (Utilities|FlowControl|Delay 0.1)
  (Camera|SetFieldOfView _camera 9e+01))

(event EventBeginPlay)

(event Collision|EventActorBeginOverlap
  (params (OtherActor :type Actor%20Object%20Reference)))

(event EventTick
  (params (DeltaSeconds :type Float%20%28single-precision%29)))

(event Input|ActionEvents|InputActionCrush
  (params (Key :type Key%20Structure))
  (bind _mesh (Variables|Character|GetMesh))
  (bind _selectedfurniture (Variables|Default|GetSelectedFurniture))
  (:Pressed
    (Utilities|IsValid _selectedfurniture
      (:Is%20Valid
        (Variables|Default|SetCapturedFurniture _selectedfurniture))))
  (:Released
    (bind _iscancontrol (CallFunction|CanControl))
    (if _iscancontrol
      (Components|Animation|PlayAnimation _mesh 0 false)
      (Utilities|IsValid (Variables|Default|GetCapturedFurniture)
        (:Is%20Valid
          (Default|Break (Variables|Default|GetCapturedFurniture) (Transformation|GetActorForwardVector)))
        (:Is%20Not%20Valid
          _))
      (Components|Animation|SetAnimationMode _mesh "AnimationBlueprint"))))

(event Input|AxisEvents|InputAxisMoveUp
  (params (AxisValue :type Float%20%28single-precision%29))
  ;[1 1 1] Moving
  (bind _iscancontrol (CallFunction|CanControl))
  (if _iscancontrol
    (CallFunction|Move AxisValue (stale Input|AxisEvents|InputAxisMoveRight AxisValue))))

(event Input|AxisEvents|InputAxisLookUp
  (params (AxisValue :type Float%20%28single-precision%29))
  ;[1 1 1] Rotation
  (bind _iscancontrol (CallFunction|CanControl))
  (if _iscancontrol
    (bind _newparam1 (CallFunction|GetYAxisValue AxisValue))
    (Transformation|AddRelativeRotation (Variables|Default|GetSpringArm) (Math|Rotator|MakeRotator 0.0 _newparam1 (stale Input|AxisEvents|InputAxisLookRight AxisValue)) false false)))

(event Input|AxisEvents|InputAxisMoveRight
  (params (AxisValue :type Float%20%28single-precision%29))
  ;[1 1 1] Moving
  (bind _iscancontrol (CallFunction|CanControl))
  (if _iscancontrol
    (CallFunction|Move (stale Input|AxisEvents|InputAxisMoveUp AxisValue) AxisValue)))

(event Input|AxisEvents|InputAxisLookRight
  (params (AxisValue :type Float%20%28single-precision%29))
  ;[1 1 1] Rotation
  (bind _iscancontrol (CallFunction|CanControl))
  (if _iscancontrol
    (Transformation|AddRelativeRotation (Variables|Default|GetSpringArm) (Math|Rotator|MakeRotator 0.0 (stale Input|AxisEvents|InputAxisLookUp _newparam1) AxisValue) false false)))

(fn ConstructionScript)

(fn GetYAxisValue
  (params (NewParam :type Float%20%28single-precision%29))
  (LocalVariables|SetCurrentY (.pitch (Variables|/Script/Engine.SceneComponent|GetRelativeRotation (Variables|Default|GetSpringArm))))
  (if (and (> (LocalVariables|GetCurrentY) -8e+01) (> 0.0 NewParam))
    (LocalVariables|SetActualAxisValue NewParam :!label _label)
    (elif (and (< 0.0 NewParam) (< (LocalVariables|GetCurrentY) 16.0))
      (goto _label)
      (else
        (LocalVariables|SetActualAxisValue 0.0))))
  (return (LocalVariables|GetActualAxisValue)))

(fn Move
  (params (XAxisValue :type Float%20%28single-precision%29) (YAxisValue :type Float%20%28single-precision%29))
  (bind _returnvalue (Math|Vector|MakeVector XAxisValue YAxisValue 0.0))
  (bind _springarm (Variables|Default|GetSpringArm))
  (bind _returnvalue_2 (Math|Conversions|RotationFromXVector _returnvalue))
  (bind _relativerotation (Variables|/Script/Engine.SceneComponent|GetRelativeRotation _springarm))
  (bind (_roll _pitch _yaw) (Math|Rotator|BreakRotator _relativerotation))
  (if (> (Math|Vector|VectorLength _returnvalue) 0.25)
    (CallFunction|ERotateto (Math|Rotator|MakeRotator (+ (.roll _returnvalue_2) _roll) (+ (.pitch _returnvalue_2) _pitch) (+ (.yaw _returnvalue_2) _yaw)))
    (Pawn|Input|AddMovementInput (Math|Conversions|ToVector(Vector2D) (Math|Vector2D|Normalize2D (Math|Conversions|ToVector2D(Vector) (Transformation|GetActorForwardVector (Pawn|GetController))))) (* (/ (+ (Math|Float|Absolute(Float) XAxisValue) (Math|Float|Absolute(Float) YAxisValue)) 2.0) (Variables|Default|GetSpeed)) false)))