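; Game mode for a chaos game: removing all registered furniture wins, and chaos decaying to zero loses.
; A looping timer drains chaos while the player has control, and each change tints a dynamic Citizen material between blue and red.
; It switches GUI frames for rules, play, win and lose, starts the citizen spawner's timer, and saves level progress to the "CE" slot.
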(event Custom|E_SpawnCitizens
  (Utilities|Time|SetTimerbyFunctionName (Variables|Default|GetCitizenSpawner) "CheckAndSpawn" 1.0 true))

(event EventBeginPlay
  (CallFunction|InitSaveGame)
  (CallFunction|InitGUI)
  (CallFunction|InitMaterial)
  (CallFunction|Pause)
  (Utilities|Time|SetTimerbyFunctionName self "DecreaseChaos" 0.2 true))

(event EventTick
  (params (DeltaSeconds :type Float%20%28single-precision%29)))

(fn ConstructionScript)

(fn AddChaos
  (params (ChaosValue :type Integer))
  (if (> (Math|Conversions|ToFloat(Integer) (Variables|Default|GetMaxChaosLevel)) (Variables|Default|GetChaosLevel))
    (Variables|Default|SetChaosLevel (+ (Math|Conversions|ToFloat(Integer) ChaosValue) (Variables|Default|GetChaosLevel)))
    (CallFunction|ChangeChaosColor)))

(fn DecreaseChaos
  (CallFunction|LowerChaos 0.1))

(fn InitMaterial
  (bind _returnvalue (Rendering|Material|CreateDynamicMaterialInstance "/Game/Materials/Citizen.Citizen" :!class /Script/Engine.KismetMaterialLibrary))
  (Variables|Default|SetMaterial _returnvalue))

(fn ChangeChaosColor
  (bind _percent (CallFunction|GetChaosPercent))
  (Variables|Default|SetChaosColor (Math|Conversions|ToColor(LinearColor) (Math|Color|MakeColor _percent 0.0 (- 1.0 _percent))))
  (Rendering|Material|SetVectorParameterValue (Variables|Default|GetMaterial) "Color" (Math|Color|MakeColor _percent 0.0 (- 1.0 _percent)) :!class /Script/Engine.MaterialInstanceDynamic))

(fn GetChaosPercent
  (return (/ (Variables|Default|GetChaosLevel) (Math|Conversions|ToFloat(Integer) (Variables|Default|GetMaxChaosLevel)))))

(fn LowerChaos
  (params (ChaosValue :type Float%20%28single-precision%29))
  (if (and (< 0.0 (Variables|Default|GetChaosLevel)) (Variables|Default|GetCanControl))
    (Variables|Default|SetChaosLevel (- (Variables|Default|GetChaosLevel) ChaosValue))
    (CallFunction|ChangeChaosColor)
    (if (<= (Variables|Default|GetChaosLevel) 0.0)
      (CallFunction|End))))

(fn Pause
  (Variables|Default|SetCanControl false)
  (Default|ShowFrame (Variables|Default|GetGUI) "/Game/UI/Rules.Rules_C")
  (Variables|/Script/Engine.PlayerController|SetbShowMouseCursor (Game|GetPlayerController 0) true))

(fn Unpause
  (Variables|Default|SetCanControl true)
  (Default|ShowFrame (Variables|Default|GetGUI) "/Game/UI/PlayWidget.PlayWidget_C")
  (Variables|/Script/Engine.PlayerController|SetbShowMouseCursor (Game|GetPlayerController 0) false))

(fn End
  (Variables|Default|SetCanControl false)
  (Default|ShowFrame (Variables|Default|GetGUI) "/Game/UI/Lose.Lose_C")
  (Variables|/Script/Engine.PlayerController|SetbShowMouseCursor (Game|GetPlayerController 0) true))

(fn InitGUI
  (bind _returnvalue (Game|SpawnActorfromClass "/Game/UI/CE_GUI.CE_GUI_C" (Math|Transform|MakeTransform "0, 0, 0") "Undefined" 0 0))
  (Variables|Default|SetGUI _returnvalue))

(fn CheckLevel
  (params (Force :type Boolean))
  (if (> (Variables|/Game/Blueprints/CE_SaveGame.CE_SaveGame_C|GetCurrentLevel (Variables|Default|GetSaveGameInstanc)) 3)
    (bind _output_get (Variables|/Game/Blueprints/CE_SaveGame.CE_SaveGame_C|SetCurrentLevel (Variables|Default|GetSaveGameInstanc) 3)))
  (bind _returnvalue (Game|GetCurrentLevelName true))
  (if (or (not (Utilities|Enum|Equal(Enum) _returnvalue (Utilities|Select :Index _output_get :Option%200 "Level0" :Option%201 "Level1" :Option%202 "Level2" :Option%203 "Level3"))) Force)
    (Game|OpenLevel(byName) (Utilities|String|StringToName (Utilities|Select :Index _output_get :Option%200 "Level0" :Option%201 "Level1" :Option%202 "Level2" :Option%203 "Level3")))))

(fn AddFurniture
  (params (Furn :type C%20Base%20Furniture%20Object%20Reference))
  (Utilities|Array|AddUnique (Variables|Default|GetFurnitures) Furn))

(fn RemoveFurniture
  (params (Furn :type C%20Base%20Furniture%20Object%20Reference))
  (bind _furnitures (Variables|Default|GetFurnitures))
  (Utilities|Array|RemoveItem _furnitures Furn)
  (if (<= (Utilities|Array|Length _furnitures) 0)
    (CallFunction|Win)))

(fn Win
  (bind _savegameinstanc (Variables|Default|GetSaveGameInstanc))
  (Variables|Default|SetCanControl false)
  (bind _result (Math|Integer|IncrementInt (Variables|/Game/Blueprints/CE_SaveGame.CE_SaveGame_C|GetCurrentLevel _savegameinstanc))
    (:%20%20
      (Variables|/Game/Blueprints/CE_SaveGame.CE_SaveGame_C|SetCurrentLevel _savegameinstanc _result)
      (SaveGame|SaveGametoSlot _savegameinstanc "CE")
      (Default|ShowFrame (Variables|Default|GetGUI) "/Game/UI/Win.Win_C")
      (Variables|/Script/Engine.PlayerController|SetbShowMouseCursor (Game|GetPlayerController 0) true))))

(fn RandomFurniturePoint
  (bind _furnitures (Variables|Default|GetFurnitures))
  (bind _returnvalue (Utilities|Array|Length _furnitures))
  (if (> _returnvalue 0)
    (Utilities|IsValid (Utilities|Array|Get(acopy) _furnitures (Math|Random|RandomIntegerinRange 0 _returnvalue))
      (:Is%20Not%20Valid
        (bind _point (Default|GetPoint (Variables|Default|GetCitizenSpawner)))
        (return _point)))
    (else
      (return (Math|Vector|MakeVector 0.0 0.0 0.0)))))

(fn InitSpawner
  (params (Spawner :type CE%20Citizen%20Spawner%20Object%20Reference))
  (Variables|Default|SetCitizenSpawner Spawner)
  (CallFunction|ESpawnCitizens)
  (return))

(fn UpdateMusic)

(fn InitSaveGame
  (bind _returnvalue (SaveGame|LoadGamefromSlot "CE"))
  (bind _asce_save_game (Utilities|Casting|CastToCE_SaveGame _returnvalue)
    (:then
      (Variables|Default|SetSaveGameInstanc _asce_save_game))
    (:CastFailed
      (bind _returnvalue_2 (SaveGame|CreateSaveGameObject "/Game/Blueprints/CE_SaveGame.CE_SaveGame_C"))
      (bind _output_get (Variables|Default|SetSaveGameInstanc _returnvalue_2))
      (SaveGame|SaveGametoSlot _output_get "CE"))))

(fn Reset
  (bind _savegameinstanc (Variables|Default|GetSaveGameInstanc))
  (Variables|/Game/Blueprints/CE_SaveGame.CE_SaveGame_C|SetCurrentLevel _savegameinstanc 0)
  (SaveGame|SaveGametoSlot _savegameinstanc "CE"))